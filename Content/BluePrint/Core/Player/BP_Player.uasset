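; BP_Player is the player Blueprint, handling a networked attack action.
; Attack passes through client-to-server and server-to-multicast events, named C2S and S2M, with the Move state checked both locally and in C2S.
; The multicast event sets State to Attack and plays the AM_Attack montage on the mesh.
; The graph shows no return to Move, and the construction script is empty.
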(event Custom|S2M_Attack
  (Variables|Default|SetState "NewEnumerator1")
  (Animation|Montage|PlayMontage (Variables|Character|GetMesh) "/Game/BluePrint/Animation/AM_Attack.AM_Attack"))

(event Custom|Attack
  (switch Utilities|FlowControl|Switch|SwitchonEN_State (Variables|Default|GetState)
    (:NewEnumerator0
      (CallFunction|C2SAttack))))

(event Custom|C2S_Attack
  (switch Utilities|FlowControl|Switch|SwitchonEN_State (Variables|Default|GetState)
    (:NewEnumerator0
      (CallFunction|S2MAttack))))

(fn ConstructionScript)