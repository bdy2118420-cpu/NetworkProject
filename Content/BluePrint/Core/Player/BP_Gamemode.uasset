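; Game mode that populates the level with NPCs and traps and applies trap effects to players.
; Shortly after BeginPlay it spawns fixed batches of BP_NPC, BP_Slow and BP_Jump at random reachable navmesh points within a radius.
; Jump and slow handlers subtract HP and pass it to the player's S2MDamage, then randomly launch the player or reduce walk speed.
; A separate handler restores walk speed when the slow effect ends.
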(event EventBeginPlay
  (Utilities|FlowControl|Delay 0.2)
  (CallFunction|SpawnNPC)
  (CallFunction|SpawnSlowTrap)
  (CallFunction|SpawnJumpTrap))

(event EventTick
  (params (DeltaSeconds :type Float%20%28single-precision%29)))

(fn ConstructionScript)

(fn SpawnNPC
  (bind (_randomlocation _returnvalue) (AI|Navigation|GetRandomReachablePointinRadius (Math|Vector|MakeVector 0.0 0.0 9e+01) 3e+03 0 0))
  (for _index (range 1 5)
    (if _returnvalue
      (Game|SpawnActorfromClass "/Game/BluePrint/Core/NPC/BP_NPC.BP_NPC_C" (Math|Transform|MakeTransform _randomlocation "0, 0, 0" "1.000000,1.000000,1.000000") "AdjustIfPossibleButAlwaysSpawn" "MultiplyWithRoot" 0 0))))

(fn SpawnSlowTrap
  (bind (_randomlocation _returnvalue) (AI|Navigation|GetRandomReachablePointinRadius (Math|Vector|MakeVector 0.0 0.0 1.0) 3e+03 0 0))
  (for _index (range 1 3)
    (if _returnvalue
      (Game|SpawnActorfromClass "/Game/BluePrint/Core/MapObject/BP_Slow.BP_Slow_C" (Math|Transform|MakeTransform _randomlocation "0, 0, 0" "1.000000,1.000000,1.000000") "AdjustIfPossibleButAlwaysSpawn" "MultiplyWithRoot" 0 0))))

(fn SpawnJumpTrap
  (bind (_randomlocation _returnvalue) (AI|Navigation|GetRandomReachablePointinRadius (Math|Vector|MakeVector 0.0 0.0 1.0) 3e+03 0 0))
  (for _index (range 1 3)
    (if _returnvalue
      (Game|SpawnActorfromClass "/Game/BluePrint/Core/MapObject/BP_Jump.BP_Jump_C" (Math|Transform|MakeTransform _randomlocation "0, 0, 0" "1.000000,1.000000,1.000000") "AdjustIfPossibleButAlwaysSpawn" "MultiplyWithRoot" 0 0))))

(fn OnJumpTrap
  (params (Player :type BP%20Player%20Object%20Reference))
  (bind _output_get (Variables|/Game/BluePrint/Core/BP_Human.BP_Human_C|SetHP Player (- (Variables|/Game/BluePrint/Core/BP_Human.BP_Human_C|GetHP Player) 2e+01)))
  (Default|S2MDamage Player _output_get)
  (Character|LaunchCharacter Player (Math|Vector|MakeVector (Math|Random|RandomFloatinRange -1e+02 1e+02) (Math|Random|RandomFloatinRange -1e+02 1e+02) (Math|Random|RandomFloatinRange 5e+02 2e+03)) false false))

(fn OnSlowTrap
  (params (Player :type BP%20Player%20Object%20Reference))
  (bind _output_get (Variables|/Game/BluePrint/Core/BP_Human.BP_Human_C|SetHP Player (- (Variables|/Game/BluePrint/Core/BP_Human.BP_Human_C|GetHP Player) 1e+01)))
  (Variables|/Script/Engine.CharacterMovementComponent|SetMaxWalkSpeed (Variables|/Script/Engine.Character|GetCharacterMovement Player) 2e+02)
  (Default|S2MDamage Player _output_get))

(fn OffSlowTrap
  (params (Player :type BP%20Player%20Object%20Reference))
  (Variables|/Script/Engine.CharacterMovementComponent|SetMaxWalkSpeed (Variables|/Script/Engine.Character|GetCharacterMovement Player) 5e+02))