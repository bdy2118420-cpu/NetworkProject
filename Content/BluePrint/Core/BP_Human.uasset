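; BP_Human is a character with networked melee combat, health and death.
; StartAttack sphere-traces forward on the server and damages any other BP_Human it hits; EndAttack returns the state to Move.
; Damage flows through S2M events, apparently server-to-multicast, which set HP and update two HP bar widgets.
; At zero HP in Move or Attack, death disables movement and capsule collision and ragdolls the mesh.
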(event Custom|EndAttack
  (switch Utilities|FlowControl|Switch|SwitchonEN_State (Variables|Default|GetState)
    (:NewEnumerator1
      (Variables|Default|SetState "NewEnumerator0"))))

(event Custom|S2M_Death
  (bind _mesh (Variables|Character|GetMesh))
  (Utilities|FlowControl|Sequence
    (:then_0
      (Variables|Default|SetState "NewEnumerator2"))
    (:then_1
      (Pawn|Components|CharacterMovement|DisableMovement (Variables|Character|GetCharacterMovement)))
    (:then_2
      (Collision|SetCollisionEnabled (Variables|Collision|GetCapsuleComponent) "NoCollision"))
    (:then_3
      (Collision|SetCollisionEnabled _mesh "PhysicsOnly")
      (Physics|SetSimulatePhysics _mesh true))))

(event Custom|StartAttack
  (bind _returnvalue (Transformation|GetActorLocation))
  (Networking|SwitchHasAuthority
    (:Authority
      (bind _outhit (Collision|SphereTraceForObjects _returnvalue (+ _returnvalue (* (Transformation|GetActorForwardVector) (Variables|Default|GetRange))) 1e+01 (Utilities|Array|MakeArray "ObjectTypeQuery3") false 0 "None"))
      (bind _asbp_human (Utilities|Casting|CastToBP_Human (.HitActor (Collision|BreakHitResult _outhit))))
      (Game|Damage|ApplyDamage _asbp_human 5e+01 0 self))))

(event Custom|S2M_Damage
  (params (NewParam :type Float%20%28double-precision%29))
  (CallFunction|SetHpUi NewParam))

(event Game|Damage|EventAnyDamage
  (params (Damage :type Float%20%28single-precision%29) (DamageType :type Damage%20Type%20Object%20Reference) (InstigatedBy :type Controller%20Object%20Reference) (DamageCauser :type Actor%20Object%20Reference))
  (CallFunction|S2MDamage (- (Variables|Default|GetHP) Damage))
  (switch Utilities|FlowControl|Switch|SwitchonEN_State (Variables|Default|GetState)
    (:NewEnumerator0
      _)
    (:NewEnumerator1
      _))
  (if (<= (Variables|Default|GetHP) 0.0)
    (CallFunction|S2MDeath)))

(fn ConstructionScript)

(fn SetHpUi
  (params (NewParam :type Float%20%28double-precision%29))
  (bind _aswbp_hpbar (Utilities|Casting|CastToWBP_HPBar (UserInterface|GetUserWidgetObject (Variables|Default|GetWidget))))
  (Progress|SetPercent (Variables|/Game/BluePrint/UI/WBP_HPBar.WBP_HPBar_C|GetProgressBar_0 _aswbp_hpbar) (/ NewParam 1e+02))
  (bind _aswbp_hpbar_2 (Utilities|Casting|CastToWBP_HPBar (UserInterface|GetUserWidgetObject (Variables|Default|GetWidget1))))
  (Progress|SetPercent (Variables|/Game/BluePrint/UI/WBP_HPBar.WBP_HPBar_C|GetProgressBar_0 _aswbp_hpbar_2) (/ NewParam 1e+02))
  (Variables|Default|SetHP NewParam))